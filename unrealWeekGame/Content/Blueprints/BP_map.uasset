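; BP_map runs a two-player local match, handling player setup, scoring and round respawns.
; BeginPlay creates the second player, adds an input mapping for the first and displays the score widget.
; When IsRespawnStart is set, Tick clears it, waits briefly, then returns both players to spawn, resetting their trails and point lists.
; AddScore credits the opponent of the passed player, using the P1 tag, and updates the widget.
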(event `self.ReceiveBeginPlay`
  (`GameplayStatics.CreatePlayer` 1)
  (`EnhancedInputSubsystemInterface.AddMappingContext` (pcsubsystem `EnhancedInputLocalPlayerSubsystem` (`GameplayStatics.GetPlayerController` 0)) "/Game/Input/I_player1.I_player1" 0 (struct))
  (bind _returnvalue (`|CreateWidget` "/Game/UI/TextScore.TextScore_C"))
  (set `self.TextScore` _returnvalue)
  (`UserWidget.AddToViewport` _returnvalue 0))

(event `self.ReceiveTick`
  (params (DeltaSeconds :type "Float (single-precision)"))
  (if (`self.isRespawnStart`)
    (set `self.isRespawnStart` false)
    (`KismetSystemLibrary.Delay` 3.0)
    (bind _asbp_player (cast `/Game/Blueprints/BP_Player` (`GameplayStatics.GetPlayerPawn` 0)))
    (`self.Respawn` _asbp_player)
    (bind _asbp_player_2 (cast `/Game/Blueprints/BP_Player` (`GameplayStatics.GetPlayerPawn` 1)))
    (`self.Respawn` _asbp_player_2)))

(fn `AddScore`
  (params (nb :type Integer) (player :type "Actor Object Reference"))
  (if (`self.ActorHasTag` player "P1")
    (set `self.ScoreP2` (+ (`self.ScoreP2`) nb))
    (else
      (set `self.ScoreP1` (+ (`self.ScoreP1`) nb))))
  (`/Game/UI/TextScore.EditText` (`self.TextScore`) (`|FormatText` "Score P1: {ScoreP1} \n \nScore P2: {ScoreP2}" (`self.ScoreP1`) (`self.ScoreP2`))))

(fn `Respawn`
  (params (player :type "/Game/Blueprints/BP_Player Object Reference"))
  (`self.SetActorHiddenInGame` player false)
  (set `/Game/Blueprints/BP_Player.IsDead` false player)
  (`self.K2_SetActorLocationAndRotation` player (.location (`/Game/Blueprints/BP_Player.SpawnPos` player)) (.rotation (`/Game/Blueprints/BP_Player.SpawnPos` player)) false true)
  (`NiagaraComponent.ReinitializeSystem` (`/Game/Blueprints/BP_Player.trail` player))
  (`KismetArrayLibrary.Array_Clear` (`/Game/Blueprints/BP_Player.PointList` player)))

(fn `UserConstructionScript`)