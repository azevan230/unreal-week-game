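; BP_Player is a constantly forward-moving, yaw-steered player that records a trail of points and can die by crossing one, light-cycle style.
; Tick appends a trail point whenever MinDistance is covered.
; A looping timer line-traces between consecutive points, ignoring Obstacle-tagged actors, killing any BP_Player hit, including itself.
; Trace hits or overlapping Death-tagged actors hide the victim and flag respawn in the BP_map game mode.
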(event `self.ReceiveBeginPlay`
  (`KismetSystemLibrary.K2_SetTimerDelegate` (delegate `check`) 0.1 true)
  (set `self.SpawnPos` (`self.GetTransform`)))

(event `check`
  (if (not (`self.IsDead`))
    (`self.CheckCollision`)))

(event `self.ReceiveTick`
  (params (DeltaSeconds :type "Float (single-precision)"))
  (bind _pointlist (`self.PointList`))
  (if (not (`self.IsDead`))
    (`self.K2_AddActorLocalOffset` (20.0 0.0 0.0))
    (if (>= (`KismetMathLibrary.Vector_Distance` (`|GetArrayItem` _pointlist (`KismetArrayLibrary.Array_LastIndex` _pointlist)) (`SceneComponent.K2_GetComponentLocation` (`self.trail`))) (`self.MinDistance`))
      (`self.CreatePoint`))))

(event `self.ReceiveActorBeginOverlap`
  (params (OtherActor :type "Actor Object Reference"))
  (`KismetSystemLibrary.PrintString` "sa a hit")
  (for _array_element (`Actor.Tags` OtherActor)
    (if (== _array_element "Death")
      (`self.SetActorHiddenInGame` true)
      (set `self.IsDead` true)
      (bind _asbp_map (cast `/Game/Blueprints/BP_map` (`GameplayStatics.GetGameMode`)))
      (set `/Game/Blueprints/BP_map.isRespawnStart` true _asbp_map))))

(fn `CheckCollision`
  (bind _pointlist (`self.PointList`))
  (for (_array_element _array_index) _pointlist
    (if (`KismetArrayLibrary.Array_IsValidIndex` _pointlist (+ _array_index 1))
      (bind _outactors (`GameplayStatics.GetAllActorsWithTag` "Obstacle"))
      (bind (_outhit _returnvalue) (`KismetSystemLibrary.LineTraceSingle` _array_element (`|GetArrayItem` _pointlist (+ _array_index 1)) "TraceTypeQuery1" false _outactors "None" false))
      (if _returnvalue
        (bind (_bblockinghit _binitialoverlap _time _distance _location _impactpoint _normal _impactnormal _physmat _hitactor) (`GameplayStatics.BreakHitResult` _outhit))
        (`self.SetActorHiddenInGame` _hitactor true)
        (bind _asbp_player (cast `/Game/Blueprints/BP_Player` _hitactor))
        (set `/Game/Blueprints/BP_Player.IsDead` true _asbp_player)
        (bind _asbp_map (cast `/Game/Blueprints/BP_map` (`GameplayStatics.GetGameMode`)))
        (set `/Game/Blueprints/BP_map.isRespawnStart` true _asbp_map)))))

(fn `CreatePoint`
  (`KismetArrayLibrary.Array_Add` (`self.PointList`) (`SceneComponent.K2_GetComponentLocation` (`self.trail`))))

(fn `rotationInput`
  (params (turnInput :type "Float (single-precision)"))
  (if (not (`self.IsDead`))
    (`self.K2_AddActorWorldRotation` (`KismetMathLibrary.MakeRotator` 0.0 0.0 turnInput))))

(fn `UserConstructionScript`)