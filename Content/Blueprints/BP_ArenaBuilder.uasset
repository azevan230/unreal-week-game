(fn `Build`
  (`/Engine/EditorBlueprintResources/StandardMacros.IsValid` (`self.Grid`)
    (:`Is Valid`
      (`InstancedStaticMeshComponent.ClearInstances` (`self.ISM_Walls`))
      (`KismetArrayLibrary.Array_Clear` (`self.SpawnTransforms`))
      (`KismetArrayLibrary.Array_Clear` (`self.PowerUpTransforms`))
      (bind _aspda_arena_grid (cast `/Game/ArenaTools/PDA_ArenaGrid` (`self.PDA_ArenaGrid`)))
      (bind _cellsize (`/Game/ArenaTools/PDA_ArenaGrid.CellSize` _aspda_arena_grid))
      (bind _width (`/Game/ArenaTools/PDA_ArenaGrid.Width` _aspda_arena_grid))
      (bind _height (`/Game/ArenaTools/PDA_ArenaGrid.Height` _aspda_arena_grid))
      (`SceneComponent.SetWorldScale3D` (`self.Floor`) (`KismetMathLibrary.MakeVector` (/ (* _cellsize _width) 100.0) (/ (* _height _cellsize) 100.0) 1.0))
      (`SceneComponent.K2_SetWorldLocation` (`self.Floor`) (`KismetMathLibrary.MakeVector` (* (/ _height 2) _cellsize) (* (/ _width 2) _cellsize)) false false)
      (for _index (range (+ _height 1))
        (set `self.index_Y` _index)
        (for _index_2 (range (+ _width 1))
          (set `self.index_X` _index_2)
          (switch `/Game/ArenaTools/E_ArenaCell` (`/Game/ArenaTools/PDA_ArenaGrid.GetCell` _aspda_arena_grid _index_2 _index)
            (:`NewEnumerator1`
              (bind _returnvalue (/ _cellsize 100.0))
              ; Wall
              (`InstancedStaticMeshComponent.AddInstance` (`self.ISM_Walls`) (`KismetMathLibrary.MakeTransform` (+ (`/Game/ArenaTools/PDA_ArenaGrid.CellToLocal` _aspda_arena_grid (`self.index_X`) (`self.index_Y`)) (`KismetMathLibrary.MakeVector` 0.0 0.0 (/ (`self.WallHeight`) 2.0))) (struct) (`KismetMathLibrary.MakeVector` _returnvalue _returnvalue (/ (`self.WallHeight`) 100.0))) false))
            (:`NewEnumerator2`
              (bind _vector (`/Game/ArenaTools/PDA_ArenaGrid.CellToLocal` _aspda_arena_grid (`self.index_X`) (`self.index_Y`)))
              ; Spawn
              (`KismetArrayLibrary.Array_Add` (`self.SpawnTransforms`) (`KismetMathLibrary.MakeTransform` (`KismetMathLibrary.TransformLocation` (`self.GetTransform`) _vector)))
              (`InstancedStaticMeshComponent.AddInstance` (`self.ISM_SpawnMarker`) (`KismetMathLibrary.MakeTransform` _vector (`KismetMathLibrary.MakeRotator` 0.0 -90.0)) false))
            (:`NewEnumerator3`
              ; Power Up
              (`KismetArrayLibrary.Array_Add` (`self.PowerUpTransforms`) (`KismetMathLibrary.MakeTransform` (`KismetMathLibrary.MakeVector` (`KismetMathLibrary.Conv_IntToDouble` (`self.index_X`)) (`KismetMathLibrary.Conv_IntToDouble` (`self.index_Y`)))))
              (`InstancedStaticMeshComponent.AddInstance` (`self.ISM_PowerUpMarkers`) (`KismetMathLibrary.MakeTransform` _vector) false))))))
    (:`Is Not Valid`
      (`AddComponent|NODE_AddReturnResultsTerminal-1`))))

(fn `Rebuild`
  (`self.Build`))

(fn `UserConstructionScript`
  (`self.Build`))